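; Humvee actor for the Tunnel movie scene that fakes driving motion on its meshes.
; Every tick it spins two meshes around their roll axis at a constant rate, independent of travel speed.
; The main mesh sways, bobs and yaws slightly using sine and cosine waves driven by its world Y position.
; A random phase offset chosen at BeginPlay keeps instances from moving in sync.
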(event `self.ReceiveBeginPlay`
  (set `self.NewVar` (`KismetMathLibrary.RandomFloatInRange` 0.0 10000.0)))

(event `self.ReceiveTick`
  (params (DeltaSeconds :type "Float (single-precision)"))
  (bind _staticmesh (`self.StaticMesh`))
  (bind (_returnvalue_x _returnvalue_y) (`KismetMathLibrary.BreakVector` (`SceneComponent.K2_GetComponentLocation` (`self.StaticMesh`))))
  (bind _returnvalue (+ _returnvalue_y (`self.NewVar`)))
  (bind _returnvalue_2 (* _returnvalue 0.007))
  (`SceneComponent.K2_AddLocalRotation` (`self.StaticMesh2`) (`KismetMathLibrary.MakeRotator` (* DeltaSeconds 100.0)) false false)
  (`SceneComponent.K2_AddLocalRotation` (`self.StaticMesh1`) (`KismetMathLibrary.MakeRotator` (* DeltaSeconds 100.0)) false false)
  (`SceneComponent.K2_SetRelativeLocation` _staticmesh (`KismetMathLibrary.MakeVector` (* (`KismetMathLibrary.Sin` _returnvalue_2) 5.0) 0.0 (+ (* (`KismetMathLibrary.Sin` (* _returnvalue 0.02)) 0.75) 100.0)) false false)
  (`SceneComponent.K2_SetRelativeRotation` _staticmesh (`KismetMathLibrary.MakeRotator` 0.0 0.0 (* (`KismetMathLibrary.Cos` _returnvalue_2) 0.5)) false false))

(fn `UserConstructionScript`)